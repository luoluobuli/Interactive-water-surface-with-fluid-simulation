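; Snow trail draw board that records the player's path into a height-field render target.
; Each tick it copies RT_HeightField to a temp target, redraws it offset by canvas movement, then stamps a yaw-rotated logo texture at the player's position.
; It publishes canvas bounds to MPC_Snow and fits a debug plane to them.
; Texel-snapped player following is multiplied by zero, pinning the canvas at the origin.
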(event EventBeginPlay
  (bind _canvassize (Variables|Default|GetCanvasSize))
  (bind _canvaspos (Variables|Default|GetCanvasPos))
  (Rendering|ClearRenderTarget2D "/Game/PhysicsSim/Snow/RT_HeightField.RT_HeightField")
  (Rendering|Material|SetVectorParameterValue "/Game/PhysicsSim/Snow/MPC_Snow.MPC_Snow" "PositionAndSize" (Math|Color|MakeColor (.x _canvaspos) (.y _canvaspos) (.x _canvassize) (.y _canvassize)) :!class /Script/Engine.KismetMaterialLibrary))

(event Collision|EventActorBeginOverlap
  (params (OtherActor :type Actor%20Object%20Reference)))

(event EventTick
  (params (DeltaSeconds :type Float%20%28single-precision%29))
  (bind _returnvalue (Game|Player|GetPlayerPawn 0))
  (bind _prevcanvaspos (Variables|Default|GetPrevCanvasPos))
  (bind _canvaspos (Variables|Default|GetCanvasPos))
  (bind _canvassize (Variables|Default|GetCanvasSize))
  (bind _returnvalue_2 (Transformation|GetActorLocation _returnvalue))
  (bind _returnvalue_3 (- _canvaspos _prevcanvaspos))
  (bind _returnvalue_4 (/ _returnvalue_3 _canvassize))
  (bind (_x _y) (Math|Vector2D|BreakVector2D _returnvalue_4))
  (CallFunction|UpdateCanvaPos (Math|Conversions|ToVector2D(Vector) _returnvalue_2))
  (CallFunction|CopyHeightField)
  (Rendering|ClearRenderTarget2D "/Game/PhysicsSim/Snow/RT_HeightField.RT_HeightField")
  (bind _returnvalue_5 (Rendering|Material|CreateDynamicMaterialInstance "/Game/PhysicsSim/Snow/M_DrawLastFrame.M_DrawLastFrame" "None" "None" :!class /Script/Engine.KismetMaterialLibrary))
  (Rendering|Material|SetVectorParameterValue _returnvalue_5 "Offset" (Utilities|Struct|MakeLinearColor _x _y 0.0 0.0) :!class /Script/Engine.MaterialInstanceDynamic)
  (Rendering|DrawMaterialtoRenderTarget "/Game/PhysicsSim/Snow/RT_HeightField.RT_HeightField" _returnvalue_5)
  (bind (_canvas _size _context) (Rendering|BeginDrawCanvastoRenderTarget "/Game/PhysicsSim/Snow/RT_HeightField.RT_HeightField"))
  (Canvas|DrawTexture :self _canvas :RenderTexture "/Game/Characters/Mannequins/Textures/Shared/T_UE_Logo_M.T_UE_Logo_M" :ScreenPosition (- (* _size (CallFunction|WorldtoUV _returnvalue_2)) "(X=15.000000,Y=15.000000)") :ScreenSize "(X=30.000000,Y=30.000000)" :CoordinateSize "(X=1.000000,Y=1.000000)" :Rotation (+ (.yaw (Transformation|GetActorRotation _returnvalue)) 9e+01) :PivotPoint "(X=0.500000,Y=0.500000)")
  (Rendering|EndDrawCanvastoRenderTarget _context))

(fn ConstructionScript
  (Transformation|SetWorldTransform (Variables|Default|GetDebugPlane) (Math|Transform|MakeTransform (Math|Conversions|ToVector(Vector2D) (Variables|Default|GetCanvasPos)) "0, 0, 0" (Math|Conversions|ToVector(Vector2D) (/ (Variables|Default|GetCanvasSize) "(X=100.000000,Y=100.000000)") 1.0)) false false))

(fn WorldtoUV
  (params (WorldPos :type Vector))
  (bind (_x _y) (Math|Vector|BreakVector WorldPos))
  (return (+ (/ (- (Math|Vector2D|MakeVector2D _x _y) (Variables|Default|GetCanvasPos)) (Variables|Default|GetCanvasSize)) "(X=0.500000,Y=0.500000)")))

(fn UpdateCanvaPos
  (params (CanvasPos :type Vector%202D%20Structure))
  (bind _canvassize (Variables|Default|GetCanvasSize))
  (bind _canvassize_2 (Variables|Default|GetCanvasSize))
  (bind _rtresolution (Variables|Default|GetRtResolution))
  (bind _returnvalue (/ _canvassize _rtresolution))
  (bind _returnvalue_2 (/ CanvasPos _returnvalue))
  (Variables|Default|SetPrevCanvasPos (Variables|Default|GetCanvasPos))
  (Variables|Default|SetCanvasPos (* (Math|Vector2D|MakeVector2D (Math|Conversions|ToFloat(Integer) (Math|Float|Floor (.x _returnvalue_2))) (Math|Conversions|ToFloat(Integer) (Math|Float|Floor (.y _returnvalue_2)))) ""))
  (Transformation|SetWorldTransform (Variables|Default|GetDebugPlane) (Math|Transform|MakeTransform (Math|Conversions|ToVector(Vector2D) (Variables|Default|GetCanvasPos)) "0, 0, 0" (Math|Conversions|ToVector(Vector2D) (/ (Variables|Default|GetCanvasSize) "(X=100.000000,Y=100.000000)") 1.0)) false false)
  (Rendering|Material|SetVectorParameterValue "/Game/PhysicsSim/Snow/MPC_Snow.MPC_Snow" "PositionAndSize" (Math|Color|MakeColor (.x (Variables|Default|GetCanvasPos)) (.y (Variables|Default|GetCanvasPos)) (.x _canvassize_2) (.y _canvassize_2)) :!class /Script/Engine.KismetMaterialLibrary))

(fn CopyHeightField
  (bind (_canvas _size _context) (Rendering|BeginDrawCanvastoRenderTarget "/Game/PhysicsSim/Snow/RT_HeightFieldTemp.RT_HeightFieldTemp"))
  (Canvas|DrawTexture :self _canvas :RenderTexture "/Game/PhysicsSim/Snow/RT_HeightField.RT_HeightField" :ScreenSize _size :CoordinateSize "(X=1.000000,Y=1.000000)" :BlendMode "BLEND_Opaque" :PivotPoint "(X=0.500000,Y=0.500000)")
  (Rendering|EndDrawCanvastoRenderTarget _context))