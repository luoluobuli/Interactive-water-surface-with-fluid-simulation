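; BP_FluidDrawBoard writes the player pawn's movement into a velocity render target, apparently as input for a 2D fluid simulation.
; On BeginPlay it creates a dynamic instance of M_VelocityPainter.
; Each Tick it clears RT_VelocityField, then passes the pawn's canvas-scaled XY velocity to the material as a color.
; It draws that material as a StrokeSize stamp at the pawn's world XY, mapped through CanvasCenter and CanvasSize.
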(event EventBeginPlay
  (bind _returnvalue (Rendering|Material|CreateDynamicMaterialInstance "/Game/PhysicsSim/Fluid2D/M_VelocityPainter.M_VelocityPainter" "None" "None" :!class /Script/Engine.KismetMaterialLibrary))
  (Variables|Default|SetVelocityPainter _returnvalue))

(event Collision|EventActorBeginOverlap
  (params (OtherActor :type Actor%20Object%20Reference)))

(event EventTick
  (params (DeltaSeconds :type Float%20%28single-precision%29))
  (bind _returnvalue (Game|Player|GetPlayerPawn 0))
  (bind _velocitypainter (Variables|Default|GetVelocityPainter))
  (bind _canvassize (Variables|Default|GetCanvasSize))
  (bind _returnvalue_2 (Transformation|GetActorLocation _returnvalue))
  (bind _returnvalue_3 (Transformation|GetVelocity _returnvalue))
  (bind (_x _y) (Math|Vector|BreakVector _returnvalue_2))
  (bind (_x_2 _y_2) (Math|Vector|BreakVector _returnvalue_3))
  (bind _returnvalue_4 (Math|Vector2D|MakeVector2D _x_2 _y_2))
  (bind _returnvalue_5 (/ _returnvalue_4 _canvassize))
  (bind (_x_3 _y_3) (Math|Vector2D|BreakVector2D _returnvalue_5))
  (Rendering|ClearRenderTarget2D "/Game/PhysicsSim/Fluid2D/RT_VelocityField.RT_VelocityField")
  (Utilities|IsValid _returnvalue
    (:Is%20Valid
      (Rendering|Material|SetVectorParameterValue _velocitypainter "Velocity" (Math|Color|MakeColor _x_3 _y_3 1.0) :!class /Script/Engine.MaterialInstanceDynamic)
      (bind (_canvas _size _context) (Rendering|BeginDrawCanvastoRenderTarget "/Game/PhysicsSim/Fluid2D/RT_VelocityField.RT_VelocityField"))
      (Canvas|DrawMaterial :self _canvas :RenderMaterial _velocitypainter :ScreenPosition (- (* (+ (/ (- (Math|Vector2D|MakeVector2D _x _y) (Variables|Default|GetCanvasCenter)) _canvassize) "(X=0.500000,Y=0.500000)") _size) (* (* (/ (Variables|Default|GetStrokeSize) _canvassize) _size) "(X=0.500000,Y=0.500000)")) :ScreenSize (* (/ (Variables|Default|GetStrokeSize) _canvassize) _size) :CoordinateSize "(X=1.000000,Y=1.000000)" :PivotPoint "(X=0.500000,Y=0.500000)")
      (Rendering|EndDrawCanvastoRenderTarget _context))))

(fn ConstructionScript)