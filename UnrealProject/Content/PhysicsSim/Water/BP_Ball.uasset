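; BP_Ball is a physics-sim water actor with a sphere mesh and a 2D wind painter component.
; The construction script registers Sphere1 as the wind sphere of the EISWindPainterComponent2D.
; When FollowPlayer is set, Tick hides the Sphere and moves the actor to the first player pawn's location each frame, without sweep or teleport.
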(event EventBeginPlay)

(event Collision|EventActorBeginOverlap
  (params (OtherActor :type Actor%20Object%20Reference)))

(event EventTick
  (params (DeltaSeconds :type Float%20%28single-precision%29))
  (bind _followplayer (Variables|StaticPainter|GetFollowPlayer))
  (if _followplayer
    (Rendering|SetVisibility (Variables|Default|GetSphere) (not _followplayer) false)
    (Transformation|SetActorLocation (Transformation|GetActorLocation (Game|Player|GetPlayerPawn 0)) false false)))

(fn ConstructionScript
  (Default|SetWindSphere (Variables|Default|GetEIS_WindPainterComponent_2D) (Variables|Default|GetSphere1)))